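; BP_Phantom is an AI enemy with a melee kill zone and a rotating scanner.
; When the player enters MeleeDetection, it disables their input and prints "Dead".
; ScannerEvent shows the laser, box and spotlight while a timeline feeds yaw deltas to ScannerFunction to rotate the laser, then hides them and prints a failure message.
; Scanner detection is unfinished: the box overlap is empty and the "Found player" check is disconnected.
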(event `self.MeleeDetection.OnComponentBeginOverlap`
  (params (OverlappedComponent :type "PrimitiveComponent Object Reference") (OtherActor :type "Actor Object Reference") (OtherComp :type "PrimitiveComponent Object Reference") (OtherBodyIndex :type Integer) (bFromSweep :type Boolean) (SweepResult :type "HitResult Structure (by ref)"))
  ;[1 1 1] Attack mode/jump scare mode
  (if (== OtherActor (cast `/Game/FirstPerson/Blueprints/BP_FirstPersonCharacter` (`GameplayStatics.GetPlayerCharacter` 0) :!pure true))
    (`self.DisableInput` (`GameplayStatics.GetPlayerCharacter` 0) (`GameplayStatics.GetPlayerController` 0))
    (`KismetSystemLibrary.PrintString` "Dead" true true (struct :`G` 0.66 :`B` 1.0 :`A` 1.0) 5.0)))

(event `ScannerEvent`
  (bind _laser (`self.Laser`))
  ;[1 1 1] Scanner rotation and appearance
  (`SceneComponent.SetVisibility` _laser true false)
  (`SceneComponent.SetVisibility` (`self.Box`) true false)
  (`SceneComponent.SetVisibility` (`self.SpotLight`) true false)
  (set `self.IsMeshVisable` true)
  (bind (_direction _rotation) (`Timeline|RotationAnimation` :!via `PlayFromStart`)
    (:`Update`
      (`self.ScannerFunction` (`self.Laser`) (.z _rotation)))
    (:`Finished`
      (`SceneComponent.SetVisibility` _laser false false)
      (`SceneComponent.SetVisibility` (`self.Box`) false false)
      (`SceneComponent.SetVisibility` (`self.SpotLight`) false false)
      (set `self.IsMeshVisable` false)
      (`KismetSystemLibrary.PrintString` "Didnt Find Player"))))

(event `self.Box.OnComponentBeginOverlap`
  (params (OverlappedComponent :type "PrimitiveComponent Object Reference") (OtherActor :type "Actor Object Reference") (OtherComp :type "PrimitiveComponent Object Reference") (OtherBodyIndex :type Integer) (bFromSweep :type Boolean) (SweepResult :type "HitResult Structure (by ref)")))

(fn `ScannerFunction`
  (params (Target :type "SceneComponent Object Reference") (`Z (Yaw)` :type "Float (single-precision)"))
  (bind (_returnvalue_roll _returnvalue_pitch _returnvalue_yaw) (`KismetMathLibrary.BreakRotator` (`KismetMathLibrary.MakeRotator` 0.0 0.0 `Z (Yaw)`)))
  (`SceneComponent.K2_AddRelativeRotation` Target (`KismetMathLibrary.MakeRotator` 0.0 0.0 _returnvalue_yaw) false false))

(fn `UserConstructionScript`)