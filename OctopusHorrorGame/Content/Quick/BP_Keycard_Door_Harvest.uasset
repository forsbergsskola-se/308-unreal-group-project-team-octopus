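; Keycard door Blueprint that swings open and closed when OpenDoor is called, provided it is not locked.
; A FlipFlop alternates between playing and reversing a timeline that lerps the door mesh yaw through a quarter turn.
; The construction script calls UpdateLightColor, which tints a rect light with the locked or unlocked color based on DoorLocked.
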(event `Open Door`
  (if (not (`self.Door Locked`))
    (`/Engine/EditorBlueprintResources/StandardMacros.FlipFlop`
      (:`A`
        (bind (_direction _doortrack) (`Timeline|Timeline` :!via `PlayFromStart` :!label _label)
          (:`Update`
            (`SceneComponent.K2_SetRelativeRotation` (`self.SM_Door`) (`KismetMathLibrary.MakeRotator` 0.0 0.0 (`KismetMathLibrary.Lerp` 0.0 90.0 _doortrack)) false false))))
      (:`B`
        (goto _label :!via `Reverse`)))))

(fn `UpdateLightColor`
  ;[1 1 1] Set Initial Light Color
  (if (`self.Door Locked`)
    (`LightComponent.SetLightColor` (`self.RectLight`) (`self.Color Locked`) true)
    (else
      (`LightComponent.SetLightColor` (`self.RectLight`) (`self.Color Unlocked`) true))))

(fn `UserConstructionScript`
  (`self.UpdateLightColor`))